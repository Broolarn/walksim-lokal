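; Double-door Blueprint that opens when anything begins overlapping its trigger volume (Triggervolym).
; The overlap plays the Dörrdriver timeline, whose Driver track lerps each door component's relative location between its own start and end vector variables.
; The graph has no end-overlap or reverse logic, so nothing here closes the doors again.
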(event OnComponentBeginOverlap(triggervolym)
  (params (OverlappedComponent :type Primitive%20Component%20Object%20Reference) (OtherActor :type Actor%20Object%20Reference) (OtherComp :type Primitive%20Component%20Object%20Reference) (OtherBodyIndex :type Integer) (bFromSweep :type Boolean) (SweepResult :type Hit%20Result%20Structure%20%28by%20ref%29))
  (bind _driver (Timeline|dörr-driver Play)
    (:Update
      (Transformation|SetRelativeLocation (Variables|Default|Getdörr1) (Math|Vector|Lerp(Vector) (Variables|Dörr1Setup|Getdörrstart1) (Variables|Dörr1Setup|Getdörrslut1) _driver) false false)
      (Transformation|SetRelativeLocation (Variables|Default|Getdörr2) (Math|Vector|Lerp(Vector) (Variables|dörr2setup|Getdörrstart2) (Variables|dörr2setup|Getdörr2slut) _driver) false false))))

(event EventBeginPlay)

(event Collision|EventActorBeginOverlap
  (params (OtherActor :type Actor%20Object%20Reference)))

(event EventTick
  (params (DeltaSeconds :type Float%20%28single-precision%29)))

(fn ConstructionScript)