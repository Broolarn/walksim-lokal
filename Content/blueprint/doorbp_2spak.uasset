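; Double door Blueprint that moves two door components, Dörr1 and Dörr2, when its Signal event fires.
; Signal prints a debug "passed" message and plays the Dörrdriver timeline, whose Driver track lerps each door's relative location from its start to its end vector without sweeping.
; The file has no reverse or close logic, and a "failed" print is left unconnected.
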(event Collision|EventActorBeginOverlap
  (params (OtherActor :type Actor%20Object%20Reference)))

(event EventSignal
  (Development|PrintString "passed" true true "(R=0.000000,G=0.660000,B=1.000000,A=1.000000)" 5.0)
  (bind _driver (Timeline|dörr-driver Play)
    (:Update
      (Transformation|SetRelativeLocation (Variables|Default|Getdörr1) (Math|Vector|Lerp(Vector) (Variables|Dörr1Setup|Getdörrstart1) (Variables|Dörr1Setup|Getdörrslut1) _driver) false false)
      (Transformation|SetRelativeLocation (Variables|Default|Getdörr2) (Math|Vector|Lerp(Vector) (Variables|dörr2setup|Getdörrstart2) (Variables|dörr2setup|Getdörr2slut) _driver) false false))))

(fn ConstructionScript)