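; Interactable lever (spak) that switches lab and corridor lighting and signals a target actor.
; Interact toggles IsOpened and plays a timeline tilting the lever, ignoring presses mid-animation; each timeline update drives the spotlights graph.
; Closed darkens the lab and lights corridors immediately; open sets lights group by group with staggered delays, sending SignalMessage after the lab group.
; Tick draws debug axes and a point from the lever pivot.
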(event EventBeginPlay)

(event Collision|EventActorBeginOverlap
  (params (OtherActor :type Actor%20Object%20Reference)))

(event EventInteract
  (|ChestBehavior)
  (Utilities|FlowControl|Sequence
    (:then_0
      (if (not (Variables|Default|GetbIsOpened))
        (|spotlights :!label _label)
        (Class|BpSignal|Signal(Message) (Variables|Default|GetTargetActor))
        (else
          (goto _label execute2))))))

(event EventTick
  (params (DeltaSeconds :type Float%20%28single-precision%29))
  (|CollapseGraph_0))

(fn ConstructionScript)